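; Customer actor that orders a random furniture type and color, then buys furniture brought into its trigger box.
; On the authority, it picks each order from Multi_GameStateBase at start and after every delivery, printing the names on screen.
; An overlapping BP_Furniture_Interaction earns full price through the game state's Sell for matching type and color, half for type only.
; The delivered furniture is destroyed even when it is the wrong type.
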(event OnComponentBeginOverlap(TriggerBox)
  (params (OverlappedComponent :type Primitive%20Component%20Object%20Reference) (OtherActor :type Actor%20Object%20Reference) (OtherComp :type Primitive%20Component%20Object%20Reference) (OtherBodyIndex :type Integer) (bFromSweep :type Boolean) (SweepResult :type Hit%20Result%20Structure%20%28by%20ref%29))
  (Variables|Default|GetCurrent%20Furniture
    (:then)
    (:else
      (bind _asbp_furniture_interaction (Utilities|Casting|CastToBP_Furniture_Interaction OtherActor))
      (Variables|Default|SetCurrent%20Furniture _asbp_furniture_interaction)
      (bind _returnvalue (CallFunction|FullPriceCheck))
      (if _returnvalue
        (Default|Sell (Variables|Default|GetAs%20Multi%20Game%20State%20Base) 10)
        (else
          (bind _returnvalue_2 (CallFunction|HalfPriceCheck))
          (if _returnvalue_2
            (Default|Sell (Variables|Default|GetAs%20Multi%20Game%20State%20Base) 5))))
      (Actor|DestroyActor (Variables|Default|GetCurrent%20Furniture))
      (Development|PrintString "Destroyed")
      (if (Ability|HasAuthority)
        (CallFunction|SelectRandomFurnitureandColor)))))

(event EventBeginPlay
  (bind _asmulti_game_state_base (Utilities|Casting|CastToMulti_GameStateBase (Game|GetGameState)))
  (Variables|Default|SetAs%20Multi%20Game%20State%20Base _asmulti_game_state_base)
  (if (Ability|HasAuthority)
    (CallFunction|SelectRandomFurnitureandColor)))

(fn ConstructionScript)

(fn FullPriceCheck
  (bind _current_furniture (Variables|Default|GetCurrent%20Furniture))
  (return (and (== (Utilities|GetClass _current_furniture) (Variables|Default|GetRequired%20Shape)) (== (Variables|/Game/Fifty8/Blueprints/Interaction/BP_Furniture_Interaction.BP_Furniture_Interaction_C|GetCurrent%20Color _current_furniture) (Variables|Default|GetRequired%20Color)))))

(fn HalfPriceCheck
  (bind _current_furniture (Variables|Default|GetCurrent%20Furniture))
  (return (and (== (Utilities|GetClass _current_furniture) (Variables|Default|GetRequired%20Shape)) (!= (Variables|/Game/Fifty8/Blueprints/Interaction/BP_Furniture_Interaction.BP_Furniture_Interaction_C|GetCurrent%20Color _current_furniture) (Variables|Default|GetRequired%20Color)))))

(fn SelectRandomFurnitureandColor
  (bind (_furniture_class _name) (Default|SelectRandomFurniture (Variables|Default|GetAs%20Multi%20Game%20State%20Base)))
  (Variables|Default|SetRequired%20Shape _furniture_class)
  (Development|PrintString _name true true "(R=0.000000,G=0.660000,B=1.000000,A=1.000000)" (LocalVariables|GetDuration))
  (bind (_color _name_2) (Default|SelectRandomColor (Variables|Default|GetAs%20Multi%20Game%20State%20Base)))
  (Variables|Default|SetRequired%20Color _color)
  (Development|PrintString _name_2 true true "(R=0.000000,G=0.660000,B=1.000000,A=1.000000)" (LocalVariables|GetDuration)))