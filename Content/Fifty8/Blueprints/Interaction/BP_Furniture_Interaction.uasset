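; Interactable furniture actor that a player picks up and throws, toggled through local interaction.
; Pickup disables physics and collision, snaps it to the player's spring arm at quarter scale, and registers it with the player's interaction component.
; Release detaches it, restores scale, collision and physics, clears that reference and applies force along the camera's forward vector.
; Server interaction only calls the parent; a game-state purchase call is left unconnected.
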(event EventBeginPlay
  (|CallParentFunction)
  (Variables|Default|SetStart%20Scale (Class|Actor|GetActorRelativeScale3D)))

(event Collision|EventActorBeginOverlap
  (params (OtherActor :type Actor%20Object%20Reference))
  (|CallParentFunction OtherActor) ; This node is disabled and will not be called.\nDrag off pins to build functionality.
)

(event EventTick
  (params (DeltaSeconds :type Float%20%28single-precision%29))
  (|CallParentFunction DeltaSeconds) ; This node is disabled and will not be called.\nDrag off pins to build functionality.
)

(fn ConstructionScript
  (|CallParentFunction))

(fn HandleLocalInteraction
  (params (Player%20That%20Interacts :type BP%20First%20Person%20Character%20Object%20Reference))
  (|CallParentFunction Player%20That%20Interacts)
  (Variables|Default|SetPlayer%20That%20Interacts Player%20That%20Interacts)
  (if (Variables|Default|GetIs%20Attached)
    (CallFunction|DetachFurniture)
    (else
      (CallFunction|AttachFurniture))))

(fn HandleServerInteraction
  (params (Player%20That%20Interacts :type BP%20First%20Person%20Character%20Object%20Reference))
  (|CallParentFunction Player%20That%20Interacts))

(fn AttachFurniture
  (bind _player_that_interacts (Variables|Default|GetPlayer%20That%20Interacts))
  (bind _bpc_interaction (Variables|/Game/FirstPerson/Blueprints/BP_FirstPersonCharacter.BP_FirstPersonCharacter_C|GetBPC_Interaction _player_that_interacts))
  (Physics|SetSimulatePhysics (Variables|Default|GetStaticMeshTop) false)
  (Transformation|AttachComponentToComponent (Variables|/Game/FirstPerson/Blueprints/BP_FirstPersonCharacter.BP_FirstPersonCharacter_C|GetSpringArm (Variables|Default|GetPlayer%20That%20Interacts)) "None" "SnapToTarget" "SnapToTarget" "KeepWorld" false)
  (Variables|/Game/Fifty8/Blueprints/Interaction/BPC_Interaction.BPC_Interaction_C|SetCurrent%20Furniture _bpc_interaction self)
  (Variables|/Game/Fifty8/Blueprints/Interaction/BPC_Interaction.BPC_Interaction_C|SetHas%20Furniture _bpc_interaction true)
  (Transformation|SetActorScale3D (* 0.25 (Variables|Default|GetStart%20Scale)))
  (Collision|SetActorEnableCollision false)
  (Variables|Default|SetIs%20Attached true)
  (Development|PrintString "Attached"))

(fn DetachFurniture
  (bind _player_that_interacts (Variables|Default|GetPlayer%20That%20Interacts))
  (bind _bpc_interaction (Variables|/Game/FirstPerson/Blueprints/BP_FirstPersonCharacter.BP_FirstPersonCharacter_C|GetBPC_Interaction _player_that_interacts))
  (Physics|SetSimulatePhysics (Variables|Default|GetStaticMeshTop) true)
  (Transformation|DetachFromActor "KeepWorld" "KeepWorld" "KeepRelative")
  (Variables|/Game/Fifty8/Blueprints/Interaction/BPC_Interaction.BPC_Interaction_C|SetCurrent%20Furniture _bpc_interaction 0)
  (Variables|/Game/Fifty8/Blueprints/Interaction/BPC_Interaction.BPC_Interaction_C|SetHas%20Furniture _bpc_interaction false)
  (Transformation|SetActorScale3D (Variables|Default|GetStart%20Scale))
  (Collision|SetActorEnableCollision true)
  (Variables|Default|SetIs%20Attached false)
  (Development|PrintString "Detached")
  (Physics|AddForce (Variables|Default|GetStaticMeshTop) (* (Math|Vector|GetForwardVector (Variables|/Game/FirstPerson/Blueprints/BP_FirstPersonCharacter.BP_FirstPersonCharacter_C|GetFirstPersonCamera (Variables|Default|GetPlayer%20That%20Interacts))) 2.5e+04) "None" true))