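; Player interaction component that detects interactable actors from the camera and routes the Interact input to them.
; Each tick, a camera line trace caches any BPI_Interaction actor hit and shows or hides its data in WB_Interaction.
; Interact input calls Server_Interact, which messages a BP_Base_Interaction target or otherwise falls back to CurrentFurniture.
; While furniture is held, input is ignored over valid targets and goes to that furniture otherwise.
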(event Custom|Server_Interact
  (params (Target :type Object%20Object%20Reference) (Player%20That%20Interacts :type BP%20First%20Person%20Character%20Object%20Reference))
  (bind _asbp_base_interaction (Utilities|Casting|CastToBP_Base_Interaction Target)
    (:then
      (Class|BPIInteraction|Interact(Message) _asbp_base_interaction Player%20That%20Interacts true)
      (Development|PrintString "Detected"))
    (:CastFailed
      (Class|BPIInteraction|Interact(Message) (Variables|Default|GetCurrent%20Furniture) Player%20That%20Interacts true)
      (Development|PrintString "Null Detected"))))

(event Input|EnhancedActionEvents|EnhancedInputActionIA_Interact
  (params (ActionValue :type Boolean) (ElapsedSeconds :type Float%20%28double-precision%29) (TriggeredSeconds :type Float%20%28double-precision%29) (InputAction :type Input%20Action%20Object%20Reference :default "/Game/Input/Actions/IA_Interact.IA_Interact"))
  (bind _has_furniture (Variables|Default|GetHas%20Furniture))
  (bind _interact_actor (Variables|Default|GetInteract%20Actor)
    (:then
      (if (not _has_furniture)
        (bind _asbp_first_person_character (Utilities|Casting|CastToBP_FirstPersonCharacter (Components|GetOwner) :!label _label))
        (CallFunction|ServerInteract _interact_actor _asbp_first_person_character)))
    (:else
      (if _has_furniture
        (goto _label)))))

(event EventBeginPlay
  (bind _output (Utilities|GetWidgetReference "/Game/Fifty8/UI/WB_Interaction.WB_Interaction_C" 10)
    (:true
      (bind _aswb_interaction (Utilities|Casting|CastToWB_Interaction _output))
      (Variables|Default|SetAs%20WB%20Interaction _aswb_interaction))))

(event EventTick
  (params (DeltaSeconds :type Float%20%28single-precision%29))
  (CallFunction|InteractionLineTrace "None"))

(fn InteractionLineTrace
  (params (DrawDebugType :type EDrawDebugTrace%20Enum :default "None"))
  (bind (_returnvalue _outhit) (Utilities|GetDownwardLineTrace 1.0 0.0 5e+02 (Game|GetPlayerCameraManager 0))
    (:Output%20Exec
      (if _returnvalue
        (if (Utilities|DoesObjectImplementInterface (.HitActor (Collision|BreakHitResult _outhit)) "/Game/Fifty8/Blueprints/Interaction/BPI_Interaction.BPI_Interaction_C")
          (bind _output_get (Variables|Default|SetInteract%20Actor (.HitActor (Collision|BreakHitResult _outhit))))
          (bind _interaction_text (Class|BPIInteraction|GetInteractData(Message) _output_get))
          (Default|UpdateWBInteraction (Variables|Default|GetAs%20WB%20Interaction) true _interaction_text)
          (else
            (Variables|Default|GetInteract%20Actor :!label _label
              (:then
                (Variables|Default|SetInteract%20Actor 0)
                (Default|UpdateWBInteraction (Variables|Default|GetAs%20WB%20Interaction) false))
              (:else))))
        (else
          (goto _label))))))