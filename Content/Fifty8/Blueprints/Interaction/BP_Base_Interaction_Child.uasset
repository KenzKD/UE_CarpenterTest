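; Child interaction Blueprint of a base interactable, likely a test or example purchasable object with a cylinder mesh.
; Local interaction calls the parent, then halves the cylinder's relative scale on each use.
; Server interaction calls the parent, then calls Buy on the Multi_GameStateBase game state with a fixed amount, splitting visual feedback from shared-state changes.
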(event EventBeginPlay
  (|CallParentFunction) ; This node is disabled and will not be called.\nDrag off pins to build functionality.
)

(event Collision|EventActorBeginOverlap
  (params (OtherActor :type Actor%20Object%20Reference))
  (|CallParentFunction OtherActor) ; This node is disabled and will not be called.\nDrag off pins to build functionality.
)

(event EventTick
  (params (DeltaSeconds :type Float%20%28single-precision%29))
  (|CallParentFunction DeltaSeconds) ; This node is disabled and will not be called.\nDrag off pins to build functionality.
)

(fn ConstructionScript
  (|CallParentFunction))

(fn HandleLocalInteraction
  (params (Player%20That%20Interacts :type BP%20First%20Person%20Character%20Object%20Reference))
  (bind _cylinder (Variables|Default|GetCylinder))
  (|CallParentFunction Player%20That%20Interacts)
  (Transformation|SetRelativeScale3D _cylinder (* 0.5 (Variables|/Script/Engine.SceneComponent|GetRelativeScale3D _cylinder))))

(fn HandleServerInteraction
  (params (Player%20That%20Interacts :type BP%20First%20Person%20Character%20Object%20Reference))
  (|CallParentFunction Player%20That%20Interacts)
  (bind _asmulti_game_state_base (Utilities|Casting|CastToMulti_GameStateBase (Game|GetGameState)))
  (Default|Buy _asmulti_game_state_base 5))