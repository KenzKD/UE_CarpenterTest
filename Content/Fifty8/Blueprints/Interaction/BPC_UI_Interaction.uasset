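; Interaction component with server-named events for two paid player actions, chipper and paint.
; The chipper event traces downward ahead of the parent and spawns the given class at the hit location.
; The paint event detaches furniture from paint and sets the chosen color on the new furniture.
; Both charge a fixed cost through the GameState only when ground is detected, and print a debug message either way.
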(event Custom|Server%20Chipper%20Interact
  (params (Forward%20Vector%20Multiplier :type Float%20%28single-precision%29) (Parent :type Actor%20Object%20Reference) (Class%20to%20Spawn :type Actor%20Class%20Reference) (GameState :type Multi%20Game%20State%20Base%20Object%20Reference))
  (bind (_returnvalue _outhit) (Utilities|GetDownwardLineTrace Forward%20Vector%20Multiplier 1.0 2.5e+02 Parent)
    (:Output%20Exec
      (if _returnvalue
        (Game|SpawnActorfromClass Class%20to%20Spawn (Math|Transform|MakeTransform (.Location (Collision|BreakHitResult _outhit)) "0, 0, 0" "1.000000,1.000000,1.000000") "Undefined" "MultiplyWithRoot" 0 0)
        (Default|Buy GameState 5)
        (Development|PrintString "Chipper")
        (else
          (Development|PrintString "BPC UI Ground not detected"))))))

(event Custom|Server%20Paint%20Interact
  (params (Furniture%20to%20Change :type BP%20Furniture%20Interaction%20Object%20Reference) (Parent%20BP :type BP%20Paint%20Widget%20Object%20Reference) (InLinearColor :type Linear%20Color%20Structure) (Game%20State :type Multi%20Game%20State%20Base%20Object%20Reference))
  (bind (_grounddetected _new_furniture) (Default|DetachfromPaint Furniture%20to%20Change Parent%20BP))
  (if _grounddetected
    (Variables|/Game/Fifty8/Blueprints/Interaction/BP_Furniture_Interaction.BP_Furniture_Interaction_C|SetCurrent%20Color _new_furniture InLinearColor)
    (Default|Buy Game%20State 5)
    (Development|PrintString "Paint")
    (else
      (Development|PrintString "BPC UI Ground not detected"))))