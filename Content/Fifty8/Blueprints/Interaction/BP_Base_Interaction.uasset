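; Base interactable Blueprint that other interaction objects extend, exposing an Interact event and an interaction text for display.
; When the server interacts, Interact calls a server handler and a multicast event for local effects.
; Both handler functions are empty hooks, separating server logic from client-side response for child classes to fill in.
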(event Custom|Server%20Interact
  (params (Player%20That%20Interacts :type BP%20First%20Person%20Character%20Object%20Reference))
  (CallFunction|HandleServerInteraction Player%20That%20Interacts))

(event Custom|Multicast%20Local%20Interact
  (params (Player%20That%20Interacts :type BP%20First%20Person%20Character%20Object%20Reference))
  (CallFunction|HandleLocalInteraction Player%20That%20Interacts))

(event EventInteract
  (params (Player%20That%20Interacts :type BP%20First%20Person%20Character%20Object%20Reference) (Server%20Interacts? :type Boolean))
  (if Server%20Interacts?
    (CallFunction|ServerInteract Player%20That%20Interacts)
    (CallFunction|MulticastLocalInteract Player%20That%20Interacts)))

(fn ConstructionScript)

(fn HandleServerInteraction
  (params (Player%20That%20Interacts :type BP%20First%20Person%20Character%20Object%20Reference)))

(fn HandleLocalInteraction
  (params (Player%20That%20Interacts :type BP%20First%20Person%20Character%20Object%20Reference)))

(fn GetInteractData
  (return (Variables|Default|GetInteraction%20Text)))